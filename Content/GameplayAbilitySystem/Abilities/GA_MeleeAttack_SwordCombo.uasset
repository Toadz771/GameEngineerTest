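; GA_MeleeAttack_SwordCombo is a melee attack ability for a sword combo, extending a parent ability that provides montage and hit-scan hooks.
; When the montage starts, it listens for gameplay events that open and close the combo window and report input.
; Input inside the window increments the combo count when the window closes; otherwise the ability ends.
; Each hit scan sets damage magnitude proportional to the combo count.
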(event `self.K2_ActivateAbility`
  (`parent.K2_ActivateAbility`)
  (`self.K2_CommitAbilityCost` false))

(event `self.Montage Started`
  (set `self.ComboCount` 1)
  (`AbilityTask_WaitGameplayEvent.WaitGameplayEvent` (struct :`TagName` "Event.ContinueCombo.Start") null
    (:`then`
      (`AbilityTask_WaitGameplayEvent.WaitGameplayEvent` (struct :`TagName` "Event.ContinueCombo.End") null
        (:`then`
          (`AbilityTask_WaitGameplayEvent.WaitGameplayEvent` (struct :`TagName` "Event.ContinueCombo.Input") null
            (:`EventReceived`
              (set `self.ReceivedInput` (`self.IsWithinComboWindow`)))))
        (:`EventReceived`
          (set `self.IsWithinComboWindow` false)
          (if (`self.ReceivedInput`)
            (`/Engine/EditorBlueprintResources/StandardMacros.IncrementInt` (`self.ComboCount`))
            (else
              (`self.K2_EndAbility`))))))
    (:`EventReceived`
      (set `self.IsWithinComboWindow` true)
      (set `self.ReceivedInput` false))))

(event `self.Handle Hit Scan Start`
  (set `self.Damage Magnitude` (* -10.0 (`self.ComboCount`)))
  (`parent.Handle Hit Scan Start`))